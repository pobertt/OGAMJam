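; BP_Door is an interactable door that opens, closes and can be locked behind a key.
; Interact tries to unlock a locked door, otherwise toggles it, animating the mesh with MoveComponentTo rotation and tracking Open and InProgress state.
; Unlocking checks the player's KeyRing for DoorKeyID, showing an Unlocked widget on success and printing the result.
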(event `self.ReceiveBeginPlay`
  (bind _asbp_player_character (cast `/Game/Player/BP_PlayerCharacter` (`GameplayStatics.GetPlayerCharacter` 0)))
  (set `self.PlayerRef` _asbp_player_character))

(event `OpenDoor`
  ;[1 1 1] OpenDoor
  (if (not (`self.InProgress`))
    (set `self.InProgress` true)
    (`KismetSystemLibrary.MoveComponentTo` (`self.StaticMesh`) (`self.K2_GetActorLocation`) (struct :`Yaw` -90.0))
    (set `self.Open` true)
    (set `self.InProgress` false)))

(event `CloseDoor`
  ;[1 1 1] CloseDoor
  (if (`self.Open`)
    (set `self.InProgress` true)
    (`KismetSystemLibrary.MoveComponentTo` (`self.StaticMesh`) (`self.K2_GetActorLocation`))
    (set `self.Open` false)
    (set `self.InProgress` false)))

(event `ToggleDoor`
  ;[1 1 1] ToggleDoor
  (if (`self.Open`)
    (`self.CloseDoor`)
    (else
      (`self.OpenDoor`))))

(event `LockDoor`
  ;[1 1 1] LockDoor
  (set `self.Locked` true))

(event `UnlockDoor`
  ;[1 1 1] UnlockDoor
  (if (`KismetArrayLibrary.Array_Contains` (`/Game/Player/BP_PlayerCharacter.KeyRing` (`self.PlayerRef`)) (`self.DoorKeyID`))
    (`KismetSystemLibrary.PrintString` "Unlocked")
    (set `self.Locked` false)
    (bind _returnvalue (`|CreateWidget` "/Game/UserInterface/Player/KeyDoor/WBP_Unlocked.WBP_Unlocked_C"))
    (`UserWidget.AddToViewport` _returnvalue 0)
    (else
      (`KismetSystemLibrary.PrintString` "Locked"))))

(fn `Interact`
  (returns (SkeletalMesh :type "SkeletalMesh Object Reference"))
  (if (`self.Locked`)
    (`self.UnlockDoor`)
    (else
      (`self.ToggleDoor`)))
  (return null))

(fn `UserConstructionScript`)