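; An interactable, key-lockable dungeon door that sends the player to the level Map_JK_EXP_2.
; Interacting while locked checks the player's KeyRing for DoorKeyID and, on a match, unlocks and plays a HUD animation.
; Otherwise it toggles: opening loads the level and sets the player's AfterDungeon flag, closing rotates the mesh.
; The swing-open and level-instance logic is disconnected; the construction script applies the configurable DoorMesh.
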(event `self.ReceiveBeginPlay`
  (bind _asbp_player_character (cast `/Game/Player/BP_PlayerCharacter` (`GameplayStatics.GetPlayerCharacter` 0)))
  (set `self.PlayerRef` _asbp_player_character))

(event `OpenDoor`
  (`GameplayStatics.OpenLevel` "Map_JK_EXP_2")
  (set `/Game/Player/BP_PlayerCharacter.AfterDungeon` true (`self.PlayerRef`)))

(event `CloseDoor`
  (bind (_returnvalue_roll _returnvalue_pitch _returnvalue_yaw) (`KismetMathLibrary.BreakRotator` (`self.K2_GetActorRotation`)))
  ;[1 1 1] CloseDoor
  (if (`self.Open`)
    (set `self.InProgress` true)
    (`KismetSystemLibrary.MoveComponentTo` (`self.StaticMesh`) (`self.K2_GetActorLocation`) (`KismetMathLibrary.MakeRotator` 0.0 0.0 (+ _returnvalue_yaw 90.0)))
    (set `self.Open` false)
    (set `self.InProgress` false)))

(event `ToggleDoor`
  ;[1 1 1] ToggleDoor
  (if (`self.Open`)
    (`self.CloseDoor`)
    (else
      (`self.OpenDoor`))))

(event `LockDoor`
  ;[1 1 1] LockDoor
  (set `self.Locked` true))

(event `UnlockDoor`
  (bind _wbp_unlocked (`/Game/UserInterface/Player/HUD/WBP_ParentHUD.WBP_Unlocked` (`/Game/Player/BP_PlayerCharacter.ParentHUDRef` (`self.PlayerRef`))))
  ;[1 1 1] UnlockDoor
  (if (`KismetArrayLibrary.Array_Contains` (`/Game/Player/BP_PlayerCharacter.KeyRing` (`self.PlayerRef`)) (`self.DoorKeyID`))
    (`KismetSystemLibrary.PrintString` "Unlocked")
    (set `self.Locked` false)
    (`Widget.SetVisibility` _wbp_unlocked "Visible")
    (`/Game/UserInterface/Player/KeyDoor/WBP_Unlocked.UnlockedAnimation` _wbp_unlocked)
    (else
      (`KismetSystemLibrary.PrintString` "Locked"))))

(fn `Interact`
  (returns (SkeletalMesh :type "SkeletalMesh Object Reference"))
  (if (`self.Locked`)
    (`self.UnlockDoor`)
    (else
      (`self.ToggleDoor`)))
  (return null))

(fn `UserConstructionScript`
  (`StaticMeshComponent.SetStaticMesh` (`self.StaticMesh`) (`self.DoorMesh`)))