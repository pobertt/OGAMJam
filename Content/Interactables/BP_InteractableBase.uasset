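; BP_InteractableBase is a base interactable actor that can be picked up and removed from the world.
; Interact prints a debug pickup message, triggers DestroyItem and returns its skeletal and static mesh assets to the caller.
; DestroyItem waits briefly before destroying the actor.
; BeginPlay stores a player reference only if the parent actor casts to BP_PlayerCharacter, though the shown graphs never use it.
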(event `self.ReceiveBeginPlay`
  (bind _asbp_player_character (cast `/Game/Player/BP_PlayerCharacter` (`self.GetParentActor`)))
  (set `self.PlayerRef` _asbp_player_character))

(event `DestroyItem`
  (`KismetSystemLibrary.Delay` 0.2)
  (`self.K2_DestroyActor`))

(fn `Interact`
  (returns (SkeletalMesh :type "SkeletalMesh Object Reference") (StaticMesh :type "StaticMesh Object Reference"))
  (`KismetSystemLibrary.PrintString` "PickedUP")
  (`self.DestroyItem`)
  (return (`SkeletalMeshComponent.SkeletalMeshAsset` (`self.SkeletalMesh`)) (`StaticMeshComponent.StaticMesh` (`self.StaticMesh`))))

(fn `UserConstructionScript`)