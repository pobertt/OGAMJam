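; Base weapon actor for the player character's first-person guns and melee weapons, handling firing, reloading, melee attacks and damage.
; Fire runs single or looping automatic shots, using a camera trace to aim a second trace from the muzzle.
; Melee sphere-traces from the weapon along camera forward; both attacks damage only "Hittable" actors.
; Reload picks empty or partial montages and draws on the player's ammo; Equip and Stow are empty.
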(event `Equip`)

(event `Stow`)

(event `self.ReceiveBeginPlay`
  (bind _asbp_player_character (cast `/Game/Player/BP_PlayerCharacter` (`self.GetParentActor`)))
  (set `self.PlayerRef` _asbp_player_character))

(event `Fire`
  (switch `/Game/Weapons/E_FireMode` (`self.FireMode`)
    (:`NewEnumerator0`
      (`self.StartFire`)
      (`self.StopFire`))
    (:`NewEnumerator1`
      (if (`/Game/Player/BP_PlayerCharacter.Shooting?` (`self.PlayerRef`)) :!label _label
        (`self.StartFire`)
        (`KismetSystemLibrary.Delay` (`self.FireDelay`))
        (goto _label)))))

(event `Melee`
  (bind _meleeaimmontages_meleemontage (break `/Game/Weapons/WeaponStructures/S_MeleeMontages` (`self.MeleeAimMontages`)))
  (if (not (`/Game/Player/BP_PlayerCharacter.ReadyToAttack` (`self.PlayerRef`)))
    (`GameplayStatics.PlaySoundAtLocation` (`self.MeleeSound`) (`self.K2_GetActorLocation`) (struct) 1.0 1.0 0.0 null null null null)
    (`|PlayMontage` (`/Game/Player/BP_PlayerCharacter.FirstPersonMesh` (`self.PlayerRef`)) _meleeaimmontages_meleemontage
      (:`then`
        (bind _outhit (`self.MeleeHit` true))
        (bind (_bblockinghit _binitialoverlap _time _distance _location _impactpoint _normal _impactnormal _physmat _hitactor) (`GameplayStatics.BreakHitResult` _outhit))
        (if (not _bblockinghit)
          _
          (elif (`self.ActorHasTag` _hitactor "Hittable")
            (`self.Dmg` _hitactor)))))))

(event `StartFire`
  (bind _returnvalue (`self.K2_GetActorLocation`))
  (bind _firesound (`self.FireSound`))
  (bind (_gunanimmontages_firemontage _gunanimmontages_firelastmontage) (break `/Game/Weapons/WeaponStructures/S_GunMontages` (`self.GunAnimMontages`)))
  (bind _returnvalue_2 (- (`self.CurrentAmmo`) 1))
  (bind _firstpersonmesh (`/Game/Player/BP_PlayerCharacter.FirstPersonMesh` (`self.PlayerRef`)))
  (switch `/Game/Interactables/E_ItemType` (`self.ItemType`)
    (:`NewEnumerator0`
      (if (> _returnvalue_2 0)
        (`GameplayStatics.PlaySoundAtLocation` _firesound _returnvalue (struct) 1.0 1.0 0.0 null null null null)
        (`|PlayMontage` _firstpersonmesh _gunanimmontages_firemontage
          (:`then`
            (set `self.CurrentAmmo` (- (`self.CurrentAmmo`) 1) :!label _label_2)
            (bind _outhit (`self.FireHitScan` true))
            (`GameplayStatics.PlayWorldCameraShake` "/Game/CameraShake/CS_Fire.CS_Fire_C" (`self.K2_GetActorLocation` (`self.PlayerRef`)) 0.0 100.0)
            (bind (_bblockinghit _binitialoverlap _time _distance _location _impactpoint _normal _impactnormal _physmat _hitactor) (`GameplayStatics.BreakHitResult` _outhit))
            (if (not _bblockinghit)
              _
              (elif (`self.ActorHasTag` _hitactor "Hittable")
                (`self.Dmg` _hitactor)))))
        (elif (== _returnvalue_2 0)
          (`GameplayStatics.PlaySoundAtLocation` _firesound _returnvalue (struct) 1.0 1.0 0.0 null null null null)
          (`|PlayMontage` _firstpersonmesh _gunanimmontages_firelastmontage
            (:`then`
              (goto _label_2)))
          (else
            (`GameplayStatics.PlaySoundAtLocation` (`self.EmptySound`) _returnvalue (struct) 1.0 1.0 0.0 null null null null)
            (`self.StopFire`)))))))

(event `Reload`
  (bind (_gunanimmontages_firemontage _gunanimmontages_firelastmontage _gunanimmontages_reload _gunanimmontages_reloadnotfull) (break `/Game/Weapons/WeaponStructures/S_GunMontages` (`self.GunAnimMontages`)))
  (bind _firstpersonmesh (`/Game/Player/BP_PlayerCharacter.FirstPersonMesh` (`self.PlayerRef`)))
  (if (and (not (== (`self.CurrentAmmo`) (`self.MagSize`))) (not (`self.Reloading?`)))
    (set `self.Reloading?` true)
    (if (== (`self.CurrentAmmo`) 0)
      (`|PlayMontage` _firstpersonmesh _gunanimmontages_reload
        (:`OnBlendOut`
          (set `/Game/Player/BP_PlayerCharacter.AmmoCount` (`KismetMathLibrary.Clamp` (- (`/Game/Player/BP_PlayerCharacter.AmmoCount` (`self.PlayerRef`)) (`self.MagSize`)) 0 100) (`self.PlayerRef`) :!label _label_3)
          (if (< (`/Game/Player/BP_PlayerCharacter.AmmoCount` (`self.PlayerRef`)) 12)
            (set `self.CurrentAmmo` (`/Game/Player/BP_PlayerCharacter.AmmoCount` (`self.PlayerRef`)))
            (set `self.Reloading?` false)
            (else
              (set `self.CurrentAmmo` (`self.MagSize`))
              (set `self.Reloading?` false))))
        (:`OnInterrupted`
          (`KismetSystemLibrary.RetriggerableDelay` 3.0)
          (set `self.Reloading?` false)))
      (else
        (`|PlayMontage` _firstpersonmesh _gunanimmontages_reloadnotfull
          (:`OnBlendOut`
            (goto _label_3))
          (:`OnInterrupted`
            (`KismetSystemLibrary.RetriggerableDelay` 3.0)
            (set `self.Reloading?` false)))))))

(event `StopFire`)

(fn `Dmg`
  (params (HitActor :type "Actor Object Reference"))
  (switch `/Game/Interactables/E_ItemType` (`self.ItemType`)
    (:`NewEnumerator0`
      (`GameplayStatics.ApplyDamage` HitActor (`self.Damage`)))
    (:`NewEnumerator1`
      (`GameplayStatics.ApplyDamage` HitActor (`self.AttackDamage`)))))

(fn `FireHitScan`
  (params (DrawDebug :type Boolean))
  (returns (OutHit :type "HitResult Structure"))
  (bind _camera (`/Game/Player/BP_PlayerCharacter.Camera` (`self.PlayerRef`)))
  (bind _returnvalue (`SceneComponent.K2_GetComponentLocation` _camera))
  (bind _outhit (`KismetSystemLibrary.LineTraceSingle` _returnvalue (+ _returnvalue (* (`SceneComponent.GetForwardVector` _camera) (`self.Range`))) "TraceTypeQuery1" false (`|MakeArray` self (`self.PlayerRef`) :!type "Actor Object Reference")))
  (bind (_bblockinghit _binitialoverlap _time _distance _location _impactpoint _normal _impactnormal _physmat _hitactor _hitcomponent _hitbonename _bonename _hititem _elementindex _faceindex _tracestart _traceend) (`GameplayStatics.BreakHitResult` _outhit))
  (bind (_outhit_2 _returnvalue_2) (`KismetSystemLibrary.LineTraceSingle` :`Start` (`SceneComponent.GetSocketLocation` (`self.WeaponMesh`) "Muzzle") :`End` (`KismetMathLibrary.SelectVector` _location _traceend) :`TraceChannel` "TraceTypeQuery1" :`DrawDebugType` (select `bool` (`local.DrawDebug`) :`false` "ForOneFrame" :`true` "ForDuration" :!type "EDrawDebugTrace Enum")))
  (if _returnvalue_2
    (return _outhit_2)))

(fn `MeleeHit`
  (params (DrawDebug :type Boolean))
  (returns (OutHit :type "HitResult Structure"))
  (bind _returnvalue (`SceneComponent.GetSocketLocation` (`self.WeaponMesh`) "Middle"))
  (bind (_outhit _returnvalue_2) (`KismetSystemLibrary.SphereTraceSingle` _returnvalue (+ _returnvalue (* (`SceneComponent.GetForwardVector` (`/Game/Player/BP_PlayerCharacter.Camera` (`self.PlayerRef`))) (`self.AttackDistance`))) 50.0 "TraceTypeQuery1" false (`|MakeArray` self (`self.PlayerRef`) :!type "Actor Object Reference") (select `bool` (`local.DrawDebug`) :`false` "ForOneFrame" :`true` "ForDuration" :!type "EDrawDebugTrace Enum")))
  (if _returnvalue_2
    (return _outhit)))

(fn `UserConstructionScript`
  (`SkeletalMeshComponent.SetSkeletalMeshAsset` (`self.WeaponMesh`) (`self.Mesh`)))