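; Base actor for damageable environment items that play sounds when hit and are destroyed when their health runs out.
; The construction script applies the ModelPlaced mesh to the static mesh component.
; Any damage lowers Health and plays HitSound, and reaching zero destroys the actor and plays DestroySound.
; On BeginPlay it stores PlayerRef if its parent actor is a BP_PlayerCharacter, though this graph never uses it afterward.
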(event `self.ReceiveBeginPlay`
  (bind _asbp_player_character (cast `/Game/Player/BP_PlayerCharacter` (`self.GetParentActor`)))
  (set `self.PlayerRef` _asbp_player_character))

(event `self.ReceiveAnyDamage`
  (params (Damage :type "Float (single-precision)") (DamageType :type "DamageType Object Reference") (InstigatedBy :type "Controller Object Reference") (DamageCauser :type "Actor Object Reference"))
  (set `self.Health` (- (`self.Health`) Damage))
  (`GameplayStatics.PlaySoundAtLocation` (`self.HitSound`) (`self.K2_GetActorLocation`) (struct) 1.0 1.0 0.0 null null null null)
  (if (<= (`self.Health`) 0.0)
    (`self.K2_DestroyActor`)
    (`GameplayStatics.PlaySoundAtLocation` (`self.DestroySound`) (`self.K2_GetActorLocation`) (struct) 1.0 1.0 0.0 null null null null)))

(fn `UserConstructionScript`
  (`StaticMeshComponent.SetStaticMesh` (`self.StaticMesh`) (`self.ModelPlaced`)))