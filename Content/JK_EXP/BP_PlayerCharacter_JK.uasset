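; First-person player character Blueprint handling sprint, crouch, jump/landing feedback and gun or melee attacks through a child-actor weapon, initially a knife.
; A Movement state links sprint and crouch, with timelines blending capsule height and speed, and a looping sphere trace gating standing up.
; A timeline dips the view on jumps and landings, while the walk-bob timeline is unwired.
; The E key subtracts health and blends post-process desaturation, chromatic aberration and vignette.
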(event `Dip`
  (params (Speed :type "Float (double-precision)") (Strength :type "Float (double-precision)"))
  (bind (_relativelocation_x _relativelocation_y) (`KismetMathLibrary.BreakVector` (`SceneComponent.RelativeLocation` (`self.FP_Root`))))
  (`TimelineComponent.SetPlayRate` (`self.TL_Dip`) Speed)
  (set `self.DipStrength` Strength)
  (bind (_direction _dipalpha) (`Timeline|TL_Dip` :!via `PlayFromStart`)
    (:`Update`
      (set `self.DipAlpha` (* _dipalpha (`self.DipStrength`)))
      (`SceneComponent.K2_SetRelativeLocation` (`self.FP_Root`) (`KismetMathLibrary.MakeVector` _relativelocation_x _relativelocation_y (`KismetMathLibrary.Lerp` 0.0 -10.0 (`self.DipAlpha`))) false false))))

(event `JumpDip`
  (`self.Dip` 4.0 0.5)
  (`GameplayStatics.PlaySoundAtLocation` null (`self.K2_GetActorLocation`) (struct) 1.0 1.0 0.0 null null null null))

(event `LandDip`
  (bind _charactermovement (`self.CharacterMovement`))
  (bind (_returnvalue_x _returnvalue_y _returnvalue_z) (`KismetMathLibrary.BreakVector` (`CharacterMovementComponent.GetLastUpdateVelocity` _charactermovement)))
  (`self.Dip` 5.0 (`KismetMathLibrary.FClamp` (`KismetMathLibrary.NormalizeToRange` (`KismetMathLibrary.VSize` (`KismetMathLibrary.MakeVector` 0.0 0.0 _returnvalue_z)) 0.0 (`CharacterMovementComponent.JumpZVelocity` _charactermovement)) 0.0 2.0))
  (`GameplayStatics.PlaySoundAtLocation` null (`self.K2_GetActorLocation`) (struct) 1.0 1.0 0.0 null null null null))

(event `self.OnJumped`
  (`self.JumpDip`))

(event `self.OnLanded`
  (params (Hit :type "HitResult Structure (by ref)"))
  (`self.LandDip`))

(event `EnhancedInput|/Game/Player/Input/Actions/IA_Move`
  (params (ActionValue :type "Vector2D Structure") (ElapsedSeconds :type "Float (double-precision)") (TriggeredSeconds :type "Float (double-precision)") (InputAction :type "InputAction Object Reference" :default "/Game/Player/Input/Actions/IA_Move.IA_Move"))
  (:`Triggered`
    (`self.ShouldStopSprint` ActionValue_Y)))

(event `StandUp`
  (bind _basewalkspeed (`self.BaseWalkSpeed`))
  (set `self.Movement` "NewEnumerator0")
  (`|ExecutionSequence`
    (:`then_0`
      (bind (_direction _crouchalpha) (`Timeline|TL_Crouch` :!via `Reverse` :!label _label)
        (:`Update`
          (set `self.CrouchAlpha` _crouchalpha)
          (switch `/Game/Player/Enums/E_MovementMode` (`self.Movement`)
            (:`NewEnumerator0`
              (set `CharacterMovementComponent.MaxWalkSpeed` (`KismetMathLibrary.Lerp` _basewalkspeed (* _basewalkspeed 0.5) (`self.CrouchAlpha`)) (`self.CharacterMovement`) :!label _label_2))
            (:`NewEnumerator1`
              (goto _label_2))
            (:`NewEnumerator2`
              _))
          (`CapsuleComponent.SetCapsuleHalfHeight` (`self.CapsuleComponent`) (`KismetMathLibrary.Lerp` (`self.StandHeight`) (`self.CrouchHeight`) (`self.CrouchAlpha`)) true))))
    (:`then_1`
      (if (`self.SprintToggle`)
        (`self.StartSprint`)))))

(event `EnhancedInput|/Game/Player/Input/Actions/IA_Crouch`
  (params (ActionValue :type Boolean) (ElapsedSeconds :type "Float (double-precision)") (TriggeredSeconds :type "Float (double-precision)") (InputAction :type "InputAction Object Reference" :default "/Game/Player/Input/Actions/IA_Crouch.IA_Crouch"))
  (:`Started`
    (set `self.CrouchToggle` true)
    (if (`|EnumEquality` (`self.Movement`) "NewEnumerator2")
      (`self.StopSprint`))
    (if (not (`NavMovementComponent.IsFalling` (`self.CharacterMovement`)))
      (set `self.Movement` "NewEnumerator1")
      (`KismetSystemLibrary.K2_ClearAndInvalidateTimerHandle` (`self.UnCrouchTimer`))
      (goto _label)))
  (:`Completed`
    (set `self.CrouchToggle` false)
    (bind _returnvalue (`KismetSystemLibrary.K2_SetTimer` null "TryToStandUp" 0.01 true))
    (set `self.UnCrouchTimer` _returnvalue)))

(event `ShouldStopSprint`
  (params (VelocityAxis :type "Float (double-precision)"))
  (if (< VelocityAxis 0.5)
    (switch `/Game/Player/Enums/E_MovementMode` (`self.Movement`) :!label _label_3
      (:`NewEnumerator2`
        (set `self.Movement` "NewEnumerator0")
        (set `CharacterMovementComponent.MaxWalkSpeed` (`self.BaseWalkSpeed`) (`self.CharacterMovement`))))))

(event `StopSprint`
  (goto _label_3))

(event `StartSprint`
  (switch `/Game/Player/Enums/E_MovementMode` (`self.Movement`) :!label _label_4
    (:`NewEnumerator0`
      (set `self.Movement` "NewEnumerator2")
      (set `CharacterMovementComponent.MaxWalkSpeed` (* (`self.BaseWalkSpeed`) 1.5) (`self.CharacterMovement`)))))

(event `EnhancedInput|/Game/Player/Input/Actions/IA_Sprint`
  (params (ActionValue :type Boolean) (ElapsedSeconds :type "Float (double-precision)") (TriggeredSeconds :type "Float (double-precision)") (InputAction :type "InputAction Object Reference" :default "/Game/Player/Input/Actions/IA_Sprint.IA_Sprint"))
  (:`Started`
    (set `self.SprintToggle` true)
    (goto _label_4))
  (:`Completed`
    (set `self.SprintToggle` false)
    (goto _label_3)))

(event `EnhancedInput|/Game/Player/Input/Actions/IA_PrimaryAction`
  (params (ActionValue :type Boolean) (ElapsedSeconds :type "Float (double-precision)") (TriggeredSeconds :type "Float (double-precision)") (InputAction :type "InputAction Object Reference" :default "/Game/Player/Input/Actions/IA_PrimaryAction.IA_PrimaryAction"))
  (bind _returnvalue (`self.ActorHasTag` (`self.GetWeapon`) "Gun"))
  (:`Started`
    (if _returnvalue
      (if (not (`|EnumInequality` (`self.Movement`) "NewEnumerator2"))
        (`self.StopSprint`))
      (if (not (`/Game/Weapons/BP_WeaponBase.Reloading?` (`self.GetWeapon`)))
        (set `self.Shooting?` true)
        (`/Game/Weapons/BP_WeaponBase.StartFire` (`self.GetWeapon`)))
      (elif (`self.ActorHasTag` (`self.GetWeapon`) "Melee")
        (if (not (and (not (`self.ReadyToAttack`)) (`self.Attacking?`)))
          (set `self.ReadyToAttack` false)
          (set `self.Attacking?` true)
          (`/Game/Weapons/BP_WeaponBase.Melee` (`self.GetWeapon`))))))
  (:`Completed`
    (if _returnvalue
      (set `self.Shooting?` false)
      (`/Game/Weapons/BP_WeaponBase.StopFire` (`self.GetWeapon`))
      (else
        (set `self.ReadyToAttack` true)
        (set `self.Attacking?` false)))))

(event `Key|E`
  (params (Key :type "Key Structure"))
  (bind _healthcurrent (`self.HealthCurrent`))
  (bind _returnvalue (`KismetMathLibrary.MapRangeClamped` _healthcurrent 100.0 0.0 0.4 1.75))
  (bind _returnvalue_2 (`KismetMathLibrary.MapRangeClamped` _healthcurrent 100.0 0.0 1.0 0.25))
  (bind _returnvalue_3 (`KismetMathLibrary.MapRangeClamped` _healthcurrent 100.0 0.0 0.0 5.0))
  (:`Pressed`
    (set `self.HealthCurrent` (- _healthcurrent 25.0))
    (bind (_direction _ppsettings) (`Timeline|Timeline` :!via `PlayFromStart`)
      (:`Update`
        (bind _returnvalue_4 (`KismetMathLibrary.Lerp` (`self.Satu`) _returnvalue_2 _ppsettings))
        (set `PostProcessComponent.Settings` (make `PostProcessSettings` :`ColorSaturation` (`KismetMathLibrary.MakeVector4` _returnvalue_4 _returnvalue_4 _returnvalue_4 1.0) :`SceneFringeIntensity` (`KismetMathLibrary.Lerp` (`self.ChromAB`) _returnvalue_3 _ppsettings) :`VignetteIntensity` (`KismetMathLibrary.Lerp` (`self.Vign`) _returnvalue _ppsettings)) (`self.PostProcess`)))
      (:`Finished`
        (set `self.ChromAB` _returnvalue_3)
        (set `self.Vign` _returnvalue)
        (set `self.Satu` _returnvalue_2)))))

(fn `CalculateLagVec`
  (bind _returnvalue (`self.GetVelocity`))
  (bind _basewalkspeed (`self.BaseWalkSpeed`))
  (set `self.LocationLagVec` (`KismetMathLibrary.VInterpTo` (`self.LocationLagVec`) (`KismetMathLibrary.ClampVectorSize` (* (`KismetMathLibrary.MakeVector` (/ (`KismetMathLibrary.Dot_VectorVector` _returnvalue (`self.GetActorRightVector`)) _basewalkspeed) (/ (`KismetMathLibrary.Dot_VectorVector` _returnvalue (`self.GetActorForwardVector`)) (* _basewalkspeed -1.0)) (/ (`KismetMathLibrary.Dot_VectorVector` _returnvalue (`self.GetActorUpVector`)) (* (`CharacterMovementComponent.JumpZVelocity` (`self.CharacterMovement`)) -1.0))) 2.0) 0.0 4.0) (`GameplayStatics.GetWorldDeltaSeconds`) (/ (/ 1.0 (`GameplayStatics.GetWorldDeltaSeconds`)) 6.0))))

(fn `GetWeapon`
  (returns (Weapon :type "/Game/Weapons/BP_WeaponBase Object Reference"))
  (bind _asbp_weapon_base (cast `/Game/Weapons/BP_WeaponBase` (`ChildActorComponent.ChildActor` (`self.Weapon`))))
  (return _asbp_weapon_base))

(fn `TryToStandUp`
  (bind (_returnvalue_x _returnvalue_y _returnvalue_z) (`KismetMathLibrary.BreakVector` (`self.K2_GetActorLocation`)))
  (bind (_returnvalue_x_2 _returnvalue_y_2 _returnvalue_z_2) (`KismetMathLibrary.BreakVector` (`self.K2_GetActorLocation`)))
  (bind (_outhits _returnvalue) (`KismetSystemLibrary.SphereTraceMulti` (`KismetMathLibrary.MakeVector` _returnvalue_x_2 _returnvalue_y_2 (+ _returnvalue_z_2 (`self.CrouchHeight`))) (`KismetMathLibrary.MakeVector` _returnvalue_x _returnvalue_y (* (+ _returnvalue_z (`self.StandHeight`)) 1.1)) (`CapsuleComponent.CapsuleRadius` (`self.CapsuleComponent`)) "TraceTypeQuery1" false (`|MakeArray` self :!type "Actor Object Reference")))
  (if (not _returnvalue)
    (`self.StandUp`)
    (`KismetSystemLibrary.K2_ClearAndInvalidateTimerHandle` (`self.UnCrouchTimer`))))

(fn `UserConstructionScript`
  (`ChildActorComponent.SetChildActorClass` (`self.Weapon`) "/Game/Weapons/Knives/Knife1/BP_Knife1.BP_Knife1_C"))