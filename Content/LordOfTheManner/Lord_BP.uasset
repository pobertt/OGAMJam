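; Lord enemy character with sword combat, driven by montages and controlled by an AI controller.
; Montage notifies spawn and socket the sword, destroy it on sheathing, and trigger a sphere trace that damages the hit actor.
; Attack, equip and unequip completions fire dispatch calls.
; Incoming damage lowers health; death ragdolls the mesh, stops AI logic, sets the dead state and expires the actor after a delay.
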(event `self.ReceiveBeginPlay`)

(event `/Game/AI/EnemyAI_BPI.Attack`
  (bind _notifyname (`|PlayMontage` (`self.Mesh`) "/Game/Maskerader/Anims/Stable_Sword_Outward_Slash_Montage.Stable_Sword_Outward_Slash_Montage")
    (:`then`
      (switch `name` _notifyname :!label _label
        (:`Hit`
          (bind _outhit (`KismetSystemLibrary.SphereTraceSingle` :`Start` (`SceneComponent.K2_GetComponentLocation` (`self.RangeStart`)) :`End` (`SceneComponent.K2_GetComponentLocation` (`self.RangeEnd`)) :`Radius` 50.0 :`TraceChannel` "TraceTypeQuery1" :`DrawDebugType` "ForDuration"))
          (`GameplayStatics.ApplyDamage` (`.HitActor` (`GameplayStatics.BreakHitResult` _outhit)) 10.0))))
    (:`OnCompleted`
      (`self.On attack end`))
    (:`OnNotifyBegin`
      (goto _label))))

(event `/Game/AI/EnemyAI_BPI.EquipWeapon`
  (bind _notifyname (`|PlayMontage` (`self.Mesh`) "/Game/Maskerader/Anims/Withdrawing_Sword_Montage.Withdrawing_Sword_Montage")
    (:`OnCompleted`
      (`self.OnWeaponEquiped`))
    (:`OnNotifyBegin`
      (switch `name` _notifyname
        (:`CreateWeapon`
          (bind _returnvalue (`|SpawnActorFromClass` "/Game/Maskerader/Weapons/Weapon_Sword_BP.Weapon_Sword_BP_C" (`self.GetTransform`) "Undefined" "MultiplyWithRoot" null null))
          (bind _output_get (set `self.WeaponActor` _returnvalue))
          (`self.K2_AttachToComponent` _output_get (`self.Mesh`) "RightHand_Sword" "SnapToTarget" "SnapToTarget" "SnapToTarget" true)
          (set `self.IsWeildingWeapon` true))))))

(event `/Game/AI/EnemyAI_BPI.UnequipWeapon`
  (bind _notifyname (`|PlayMontage` (`self.Mesh`) "/Game/Maskerader/Anims/Sheathing_Sword_Montage.Sheathing_Sword_Montage")
    (:`OnCompleted`
      (`self.OnWeaponUnequiped`))
    (:`OnNotifyBegin`
      (switch `name` _notifyname
        (:`DestroyWeapon`
          (`self.K2_DestroyActor` (`self.WeaponActor`))
          (set `self.IsWeildingWeapon` false))))))

(event `self.ReceiveAnyDamage`
  (params (Damage :type "Float (single-precision)") (DamageType :type "DamageType Object Reference") (InstigatedBy :type "Controller Object Reference") (DamageCauser :type "Actor Object Reference"))
  (bind _isdead (`self.TakeDamage` (`KismetMathLibrary.FTrunc` Damage)))
  (`KismetSystemLibrary.PrintString` (`KismetStringLibrary.Conv_IntToString` (`self.Health`)))
  (if _isdead
    (`self.Die`)))

(fn `Die`
  (bind _mesh (`self.Mesh`))
  (`PrimitiveComponent.SetSimulatePhysics` _mesh true)
  (`PrimitiveComponent.SetCollisionEnabled` _mesh "QueryAndPhysics")
  (`BrainComponent.StopLogic` (`AIController.BrainComponent` (`AIBlueprintHelperLibrary.GetAIController` self)) "")
  (`/Game/AI/EnemeyBase_AIC.SetStateAsDead` (cast `/Game/AI/EnemeyBase_AIC` (`AIBlueprintHelperLibrary.GetAIController` self) :!pure true))
  (`self.SetLifeSpan` 4.0))

(fn `TakeDamage`
  (params (DamageAmount :type Integer))
  (returns (IsDead :type Boolean))
  (bind _returnvalue (- (`self.Health`) DamageAmount))
  (set `self.Health` _returnvalue)
  (if (<= _returnvalue 0)
    (return true)
    (else
      (return false))))

(fn `UserConstructionScript`
  (`parent.UserConstructionScript`))