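; Gun component for the first-person player that handles single or automatic firing, magazine ammo, reloading and damage.
; Fire calls StartFire, which spends ammo, plays feedback and runs FireHitScan.
; The hitscan traces from the camera, then from the muzzle toward that trace's end, damaging actors tagged Hittable or Enemy.
; Reload plays a montage and refills from the player's reserve on blend out.
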(event `self.ReceiveBeginPlay`
  (bind _asbp_player_character (cast `/Game/Player/BP_PlayerCharacter` (`GameplayStatics.GetPlayerCharacter` 0)))
  (set `self.PlayerRef` _asbp_player_character))

(event `StopFire`)

(event `Fire`
  (switch `/Game/Holdables/Weapons/Guns/E_FireMode` (`self.FireMode`)
    (:`NewEnumerator0`
      (`self.StartFire`)
      (`self.StopFire`))
    (:`NewEnumerator1`
      (if (`/Game/Player/BP_PlayerCharacter.Shooting?` (`self.PlayerRef`)) :!label _label
        (`self.StartFire`)
        (`KismetSystemLibrary.Delay` (`self.FireDelay`))
        (goto _label)))))

(event `StartFire`
  (bind _firesound (`self.FireSound`))
  (bind (_gunanimmontages_firemontage _gunanimmontages_firelastmontage) (break `/Game/Holdables/Weapons/WeaponStructures/S_GunMontages` (`self.GunAnimMontages`)))
  (bind _returnvalue (`Actor.K2_GetActorLocation` (`self.GetOwner`)))
  (bind _returnvalue_2 (`Actor.K2_GetActorLocation` (`self.GetOwner`)))
  (bind _returnvalue_3 (- (`self.CurrentAmmo`) 1))
  (bind _firstpersonmesh (`/Game/Player/BP_PlayerCharacter.FirstPersonMesh` (`self.PlayerRef`)))
  (switch `/Game/Holdables/E_ItemType` (`self.ItemType`)
    (:`NewEnumerator0`
      (if (> _returnvalue_3 0)
        (`GameplayStatics.PlaySoundAtLocation` _firesound _returnvalue (struct) 1.0 1.0 0.0 null null null null)
        (`|PlayMontage` _firstpersonmesh _gunanimmontages_firemontage
          (:`then`
            (bind _output_get (set `self.CurrentAmmo` (- (`self.CurrentAmmo`) 1) :!label _label_2))
            (set `/Game/Player/BP_PlayerCharacter.TempAmmoVal` _output_get (`self.PlayerRef`))
            (bind _outhit (`self.FireHitScan` false))
            (`GameplayStatics.PlayWorldCameraShake` "/Game/CameraShake/CS_Fire.CS_Fire_C" (`Actor.K2_GetActorLocation` (`self.PlayerRef`)) 0.0 100.0)
            (bind (_bblockinghit _binitialoverlap _time _distance _location _impactpoint _normal _impactnormal _physmat _hitactor) (`GameplayStatics.BreakHitResult` _outhit))
            (if (not _bblockinghit)
              _
              (elif (`Actor.ActorHasTag` _hitactor "Hittable")
                (`self.Dmg` _hitactor)
                (elif (`Actor.ActorHasTag` _hitactor "Enemy")
                  (`GameplayStatics.PlaySoundAtLocation` "/Game/Sound/knife-vintage-modified/stab-flesh/RandomStabFlesh.RandomStabFlesh" _returnvalue_2 (struct) 1.0 1.0 0.0 null null null null)
                  (`AISense_Hearing.ReportNoiseEvent` _returnvalue_2 1.0 (`self.PlayerRef`))
                  (`self.Dmg` _hitactor))))))
        (elif (== _returnvalue_3 0)
          (`GameplayStatics.PlaySoundAtLocation` _firesound _returnvalue (struct) 1.0 1.0 0.0 null null null null)
          (`|PlayMontage` _firstpersonmesh _gunanimmontages_firelastmontage
            (:`then`
              (goto _label_2)))
          (else
            (`GameplayStatics.PlaySoundAtLocation` (`self.EmptySound`) _returnvalue (struct) 1.0 1.0 0.0 null null null null)
            (`self.StopFire`)))))))

(event `Reload`
  (bind (_gunanimmontages_firemontage _gunanimmontages_firelastmontage _gunanimmontages_reload _gunanimmontages_reloadnotfull) (break `/Game/Holdables/Weapons/WeaponStructures/S_GunMontages` (`self.GunAnimMontages`)))
  (if (and (not (== (`self.CurrentAmmo`) (`self.MagSize`))) (not (`self.Reloading?`)))
    (set `self.Reloading?` true)
    (if (== (`self.CurrentAmmo`) 0)
      _
      (else
        _))
    (`GameplayStatics.PlaySoundAtLocation` "/Game/Sound/gun/full_reload.full_reload" (`Actor.K2_GetActorLocation` (`/Game/Player/BP_PlayerCharacter.GetWeapon` (`self.PlayerRef`))) (struct) 1.0 1.0 0.0 null null null null)
    (`|PlayMontage` (`/Game/Player/BP_PlayerCharacter.FirstPersonMesh` (`self.PlayerRef`)) _gunanimmontages_reloadnotfull
      (:`OnBlendOut`
        (`self.ReloadAmmo`))
      (:`OnInterrupted`
        (`KismetSystemLibrary.RetriggerableDelay` 3.0)
        (set `self.Reloading?` false)))))

(fn `Dmg`
  (params (HitActor :type "Actor Object Reference"))
  (switch `/Game/Holdables/E_ItemType` (`self.ItemType`)
    (:`NewEnumerator0`
      (`GameplayStatics.ApplyDamage` HitActor (`self.Damage`)))))

(fn `FireHitScan`
  (params (DrawDebug :type Boolean))
  (returns (OutHit :type "HitResult Structure"))
  (bind _camera (`/Game/Player/BP_PlayerCharacter.Camera` (`self.PlayerRef`)))
  (bind _returnvalue (`SceneComponent.K2_GetComponentLocation` _camera))
  (bind _weaponmesh (`/Game/Holdables/Weapons/BP_WeaponBase.WeaponMesh` (`/Game/Player/BP_PlayerCharacter.GetWeapon` (`self.PlayerRef`))))
  (bind _returnvalue_2 (`SceneComponent.GetSocketLocation` _weaponmesh "Muzzle"))
  (bind _outhit (`KismetSystemLibrary.LineTraceSingle` _returnvalue (+ _returnvalue (* (`SceneComponent.GetForwardVector` _camera) (`self.Range`))) "TraceTypeQuery1" false (`|MakeArray` null (`self.PlayerRef`) :!type "Actor Object Reference")))
  (bind (_bblockinghit _binitialoverlap _time _distance _location _impactpoint _normal _impactnormal _physmat _hitactor _hitcomponent _hitbonename _bonename _hititem _elementindex _faceindex _tracestart _traceend) (`GameplayStatics.BreakHitResult` _outhit))
  (bind _returnvalue_3 (`KismetMathLibrary.SelectVector` _location _traceend))
  (bind (_outhit_2 _returnvalue_4) (`KismetSystemLibrary.LineTraceSingle` :`Start` (`SceneComponent.GetSocketLocation` (`Actor.RootComponent` (`self.GetOwner`)) "Muzzle") :`End` _returnvalue_3 :`TraceChannel` "TraceTypeQuery1" :`DrawDebugType` (select `bool` (`local.DrawDebug`) :`true` "ForDuration" :!type "EDrawDebugTrace Enum")))
  (`NiagaraFunctionLibrary.SpawnSystemAttached` "/Game/FirstPerson/Muzzle_01_Converted.Muzzle_01_Converted" _weaponmesh "Muzzle" _returnvalue_2 (`KismetMathLibrary.FindLookAtRotation` _returnvalue_2 _returnvalue_3) "KeepWorldPosition" true)
  (if _returnvalue_4
    (return _outhit_2)))

(fn `ReloadAmmo`
  (if (> (+ (`self.CurrentAmmo`) (`/Game/Player/BP_PlayerCharacter.AmmoCount` (`self.PlayerRef`))) (`self.MagSize`))
    (bind _output_get (set `self.TempAmmo` (- (`self.MagSize`) (`self.CurrentAmmo`))))
    (bind _output_get_2 (set `self.CurrentAmmo` (`KismetMathLibrary.Clamp` (+ (`/Game/Player/BP_PlayerCharacter.AmmoCount` (`self.PlayerRef`)) (`self.CurrentAmmo`)) 0 (`self.MagSize`))))
    (set `/Game/Player/BP_PlayerCharacter.TempAmmoVal` _output_get_2 (`self.PlayerRef`))
    (set `self.Reloading?` false)
    (set `/Game/Player/BP_PlayerCharacter.AmmoCount` (`KismetMathLibrary.Clamp` (- (`/Game/Player/BP_PlayerCharacter.AmmoCount` (`self.PlayerRef`)) _output_get) 0 100) (`self.PlayerRef`))
    (else
      (bind _output_get_3 (set `self.CurrentAmmo` (`/Game/Player/BP_PlayerCharacter.AmmoCount` (`self.PlayerRef`))))
      (set `/Game/Player/BP_PlayerCharacter.TempAmmoVal` _output_get_3 (`self.PlayerRef`))
      (set `self.Reloading?` false)
      (set `/Game/Player/BP_PlayerCharacter.AmmoCount` 0 (`self.PlayerRef`)))))