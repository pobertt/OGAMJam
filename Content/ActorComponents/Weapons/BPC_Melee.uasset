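; Melee weapon actor component that plays the player's first-person attack montage and resolves the hit.
; As the montage starts, a sphere trace runs from the weapon's "Middle" socket along the camera's forward vector.
; Misses play a swing sound, while actor tags route hits: Hittable takes damage, Enemy adds impact sound and AI noise, and Lord gets sound and noise without damage.
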(event `self.ReceiveBeginPlay`
  (bind _asbp_player_character (cast `/Game/Player/BP_PlayerCharacter` (`GameplayStatics.GetPlayerCharacter` 0)))
  (set `self.PlayerRef` _asbp_player_character))

(event `Melee`
  (bind _meleeaimmontages_meleemontage (break `/Game/Holdables/Weapons/WeaponStructures/S_MeleeMontages` (`self.MeleeAimMontages`)))
  (bind _returnvalue (`Actor.K2_GetActorLocation` (`self.GetOwner`)))
  (switch `/Game/Holdables/E_ItemType` (`self.ItemType`)
    (:`NewEnumerator1`
      (if (not (`/Game/Player/BP_PlayerCharacter.ReadyToAttack` (`self.PlayerRef`)))
        (`|PlayMontage` (`/Game/Player/BP_PlayerCharacter.FirstPersonMesh` (`self.PlayerRef`)) _meleeaimmontages_meleemontage
          (:`then`
            (`KismetSystemLibrary.PrintString` "notify begin")
            (bind _outhit (`self.MeleeHit` true))
            (bind _output_get (set `self.OutHit` _outhit))
            (bind (_bblockinghit _binitialoverlap _time _distance _location _impactpoint _normal _impactnormal _physmat _hitactor) (`GameplayStatics.BreakHitResult` _output_get))
            (if (not _bblockinghit)
              (`GameplayStatics.PlaySoundAtLocation` (`self.MeleeSound`) (`Actor.K2_GetActorLocation` (`self.GetOwner`)) (struct) 1.0 1.0 0.0 null null null null)
              (elif (`Actor.ActorHasTag` _hitactor "Hittable")
                (`self.Dmg` _hitactor)
                (else
                  (bind _returnvalue_2 (`Actor.ActorHasTag` _hitactor "Enemy"))
                  (if (or _returnvalue_2 (`Actor.ActorHasTag` _hitactor "Lord"))
                    (`GameplayStatics.PlaySoundAtLocation` (`self.EnemyDmgSound`) _returnvalue (struct) 1.0 1.0 0.0 null null null null)
                    (`AISense_Hearing.ReportNoiseEvent` _returnvalue 1.0 (`self.PlayerRef`))
                    (if _returnvalue_2
                      (`self.Dmg` _hitactor)))))))
          (:`OnCompleted`
            (set `self.OutHit` (`GameplayStatics.MakeHitResult` false))
            (`KismetSystemLibrary.PrintString` "NOTIFY END")))))))

(fn `Dmg`
  (params (HitActor :type "Actor Object Reference"))
  (switch `/Game/Holdables/E_ItemType` (`self.ItemType`)
    (:`NewEnumerator1`
      (`GameplayStatics.ApplyDamage` HitActor (`self.AttackDamage`)))))

(fn `MeleeHit`
  (params (DrawDebug :type Boolean))
  (returns (OutHit :type "HitResult Structure"))
  (bind _returnvalue (`SceneComponent.GetSocketLocation` (`Actor.RootComponent` (`self.GetOwner`)) "Middle"))
  (bind (_outhit _returnvalue_2) (`KismetSystemLibrary.SphereTraceSingle` _returnvalue (+ _returnvalue (* (`SceneComponent.GetForwardVector` (`/Game/Player/BP_PlayerCharacter.Camera` (`self.PlayerRef`))) (`self.AttackDistance`))) 50.0 "TraceTypeQuery1" false (`|MakeArray` (`self.PlayerRef`) :!type "Actor Object Reference") (select `bool` (`local.DrawDebug`) :`false` "ForOneFrame" :`true` "ForDuration" :!type "EDrawDebugTrace Enum") true (struct :`R` 1.0 :`A` 1.0) (struct :`G` 1.0 :`A` 1.0) 0.5))
  (if _returnvalue_2
    (return _outhit)))