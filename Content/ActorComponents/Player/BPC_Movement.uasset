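; Player movement component for BP_PlayerCharacter, handling sprint, crouch and procedural first-person bob, dip and velocity lag.
; Enhanced Input toggles a Walking/Sprinting/Crouching state, with sprint scaling walk speed.
; Releasing crouch starts a looping timer that sphere-traces for headroom before standing, then resumes held sprint.
; Jump and landing play sounds and call Dip, but Dip is empty and the capsule, camera-dip and walk-bob blocks are unconnected here.
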(event `self.ReceiveBeginPlay`
  (bind _asbp_player_character (cast `/Game/Player/BP_PlayerCharacter` (`GameplayStatics.GetPlayerCharacter` 0)))
  (set `self.PlayerRef` _asbp_player_character))

(event `Dip`
  (params (Speed :type "Float (double-precision)") (Strength :type "Float (double-precision)")))

(event `JumpDip`
  (`self.Dip` 4.0 0.5)
  (`GameplayStatics.PlaySoundAtLocation` null (`Actor.K2_GetActorLocation` (`self.PlayerRef`)) (struct) 1.0 1.0 0.0 null null null null))

(event `LandDip`
  (bind _playerref (`self.PlayerRef`))
  (bind _charactermovement (`Character.CharacterMovement` _playerref))
  (bind (_returnvalue_x _returnvalue_y _returnvalue_z) (`KismetMathLibrary.BreakVector` (`CharacterMovementComponent.GetLastUpdateVelocity` _charactermovement)))
  (`self.Dip` 5.0 (`KismetMathLibrary.FClamp` (`KismetMathLibrary.NormalizeToRange` (`KismetMathLibrary.VSize` (`KismetMathLibrary.MakeVector` 0.0 0.0 _returnvalue_z)) 0.0 (`CharacterMovementComponent.JumpZVelocity` _charactermovement)) 0.0 2.0))
  (`GameplayStatics.PlaySoundAtLocation` null (`Actor.K2_GetActorLocation` _playerref) (struct) 1.0 1.0 0.0 null null null null))

(event `OnJumped`
  (`self.JumpDip`))

(event `OnLanded`
  (params (Hit :type "HitResult Structure (by ref)"))
  (`self.LandDip`))

(event `StandUp`
  (set `self.Movement` "NewEnumerator0")
  (`|ExecutionSequence`
    (:`then_1`
      (if (`self.SprintToggle`)
        (`self.StartSprint`)))))

(event `EnhancedInput|/Game/Player/Input/Actions/IA_Crouch`
  (params (ActionValue :type Boolean) (ElapsedSeconds :type "Float (double-precision)") (TriggeredSeconds :type "Float (double-precision)") (InputAction :type "InputAction Object Reference" :default "/Game/Player/Input/Actions/IA_Crouch.IA_Crouch"))
  (:`Started`
    (set `self.CrouchToggle` true)
    (if (`|EnumEquality` (`self.Movement`) "NewEnumerator2")
      (`self.StopSprint`))
    (if (not (`NavMovementComponent.IsFalling` (`Character.CharacterMovement` (`self.PlayerRef`))))
      (set `self.Movement` "NewEnumerator1")
      (`KismetSystemLibrary.K2_ClearAndInvalidateTimerHandle` (`self.UnCrouchTimer`))))
  (:`Completed`
    (set `self.CrouchToggle` false)
    (bind _returnvalue (`KismetSystemLibrary.K2_SetTimer` null "TryToStandUp" 0.01 true))
    (set `self.UnCrouchTimer` _returnvalue)))

(event `ShouldStopSprint`
  (params (VelocityAxis :type "Float (double-precision)"))
  (if (< VelocityAxis 0.5)
    (switch `/Game/Player/Enums/E_MovementMode` (`self.Movement`) :!label _label
      (:`NewEnumerator2`
        (set `self.Movement` "NewEnumerator0")
        (set `CharacterMovementComponent.MaxWalkSpeed` (`self.BaseWalkSpeed`) (`Character.CharacterMovement` (`self.PlayerRef`)))))))

(event `StopSprint`
  (goto _label))

(event `StartSprint`
  (switch `/Game/Player/Enums/E_MovementMode` (`self.Movement`) :!label _label_2
    (:`NewEnumerator0`
      (set `self.Movement` "NewEnumerator2")
      (set `CharacterMovementComponent.MaxWalkSpeed` (* (`self.BaseWalkSpeed`) 1.5) (`Character.CharacterMovement` (`self.PlayerRef`))))))

(event `EnhancedInput|/Game/Player/Input/Actions/IA_Sprint`
  (params (ActionValue :type Boolean) (ElapsedSeconds :type "Float (double-precision)") (TriggeredSeconds :type "Float (double-precision)") (InputAction :type "InputAction Object Reference" :default "/Game/Player/Input/Actions/IA_Sprint.IA_Sprint"))
  (:`Started`
    (set `self.SprintToggle` true)
    (goto _label_2))
  (:`Completed`
    (set `self.SprintToggle` false)
    (goto _label)))

(fn `CalculateLagVec`
  (bind _basewalkspeed (`self.BaseWalkSpeed`))
  (bind _playerref (`self.PlayerRef`))
  (bind _returnvalue (`Actor.GetVelocity` _playerref))
  (set `self.LocationLagVec` (`KismetMathLibrary.VInterpTo` (`self.LocationLagVec`) (`KismetMathLibrary.ClampVectorSize` (* (`KismetMathLibrary.MakeVector` (/ (`KismetMathLibrary.Dot_VectorVector` _returnvalue (`Actor.GetActorRightVector` _playerref)) _basewalkspeed) (/ (`KismetMathLibrary.Dot_VectorVector` _returnvalue (`Actor.GetActorForwardVector` _playerref)) (* _basewalkspeed -1.0)) (/ (`KismetMathLibrary.Dot_VectorVector` _returnvalue (`Actor.GetActorUpVector` _playerref)) (* (`CharacterMovementComponent.JumpZVelocity` (`Character.CharacterMovement` _playerref)) -1.0))) 2.0) 0.0 4.0) (`GameplayStatics.GetWorldDeltaSeconds`) (/ (/ 1.0 (`GameplayStatics.GetWorldDeltaSeconds`)) 6.0))))

(fn `TryToStandUp`
  (bind _playerref (`self.PlayerRef`))
  (bind (_returnvalue_x _returnvalue_y _returnvalue_z) (`KismetMathLibrary.BreakVector` (`Actor.K2_GetActorLocation` _playerref)))
  (bind (_returnvalue_x_2 _returnvalue_y_2 _returnvalue_z_2) (`KismetMathLibrary.BreakVector` (`Actor.K2_GetActorLocation` _playerref)))
  (bind (_outhits _returnvalue) (`KismetSystemLibrary.SphereTraceMulti` (`KismetMathLibrary.MakeVector` _returnvalue_x_2 _returnvalue_y_2 (+ _returnvalue_z_2 (`self.CrouchHeight`))) (`KismetMathLibrary.MakeVector` _returnvalue_x _returnvalue_y (* (+ _returnvalue_z (`self.StandHeight`)) 1.1)) (`CapsuleComponent.CapsuleRadius` (`Character.CapsuleComponent` (`self.PlayerRef`))) "TraceTypeQuery1" false (`|MakeArray` null :!type "Actor Object Reference")))
  (if (not _returnvalue)
    (`self.StandUp`)
    (`KismetSystemLibrary.K2_ClearAndInvalidateTimerHandle` (`self.UnCrouchTimer`))))