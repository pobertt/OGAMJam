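; BPC_Medkit is a medkit component that lets the player restore a fixed amount of health when below maximum.
; UseMedkit blocks repeat use, plays a sound and runs a reload montage on the first-person mesh, applying clamped healing only on completion.
; Completion, or interruption after a retriggerable delay, clears the in-use flag, removes BP_Medkit from the player's WeaponClass list and destroys the current weapon actor.
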(event `self.ReceiveBeginPlay`
  (bind _asbp_player_character (cast `/Game/Player/BP_PlayerCharacter` (`GameplayStatics.GetPlayerCharacter` 0)))
  (set `self.PlayerRef` _asbp_player_character))

(event `UseMedkit`
  (bind _playerref (`self.PlayerRef`))
  (if (and (not (`self.UsingMedkit?`)) (< (`/Game/Player/BP_PlayerCharacter.HealthCurrent` _playerref) (`/Game/Player/BP_PlayerCharacter.HealthMax` _playerref)))
    (set `self.UsingMedkit?` true)
    (`GameplayStatics.PlaySoundAtLocation` "/Game/Sound/medkit/medkit.medkit" (`Actor.K2_GetActorLocation` (`self.PlayerRef`)) (struct) 1.0 1.0 0.0 null null null null)
    (`|PlayMontage` (`/Game/Player/BP_PlayerCharacter.FirstPersonMesh` (`self.PlayerRef`)) "/Game/Player/TESTanims/FP_PS_ReloadNotFull_Montage.FP_PS_ReloadNotFull_Montage"
      (:`OnCompleted`
        (`self.AddHealth`)
        (`self.MedkitCompleted`))
      (:`OnInterrupted`
        (`KismetSystemLibrary.RetriggerableDelay` 3.0)
        (`self.MedkitCompleted`)))))

(event `MedkitCompleted`
  (bind _playerref (`self.PlayerRef`))
  (set `self.UsingMedkit?` false)
  (`KismetArrayLibrary.Array_RemoveItem` (`/Game/Player/BP_PlayerCharacter.WeaponClass` _playerref) "/Game/Holdables/Weapons/Items/Medkit/BP_Medkit.BP_Medkit_C")
  (`Actor.K2_DestroyActor` (`/Game/Player/BP_PlayerCharacter.GetWeapon` _playerref)))

(event `AddHealth`
  (bind _playerref (`self.PlayerRef`))
  (bind _healthcurrent (`/Game/Player/BP_PlayerCharacter.HealthCurrent` _playerref))
  (set `/Game/Player/BP_PlayerCharacter.HealthCurrent` (`KismetMathLibrary.FClamp` (+ _healthcurrent 25.0) 0.0 100.0) _playerref)
  (`KismetSystemLibrary.PrintString` (`KismetStringLibrary.Conv_DoubleToString` _healthcurrent)))