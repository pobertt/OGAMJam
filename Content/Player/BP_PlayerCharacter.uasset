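; First-person player character handling movement, inventory, health, interaction and UI for notes, keys, pause and game over.
; Enhanced Input drives sprint and crouch, with a looping sphere-trace timer gating stand-up and a timeline dipping the view on jumps and landings.
; Pickups and item cycling swap a socketed child-actor weapon, whose item type routes primary actions to gun, melee or medkit components.
; Damage triggers HUD effects and death.
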(event Custom|AddAmmo
  (bind _parenthudref (Variables|UI|GetParentHUDRef))
  (bind _wbp_ammoadded (Variables|/Game/UserInterface/Player/HUD/WBP_ParentHUD.WBP_ParentHUD_C|GetWBP_AmmoAdded _parenthudref))
  (Widget|SetVisibility _wbp_ammoadded "Visible")
  (Default|AmmoAddedAnimation _wbp_ammoadded))

(event Custom|AddKey
  (params (KeyID :type Integer))
  (bind _parenthudref (Variables|UI|GetParentHUDRef))
  (bind _parenthudref_2 (Variables|UI|GetParentHUDRef))
  (bind _wbp_keyadded (Variables|/Game/UserInterface/Player/HUD/WBP_ParentHUD.WBP_ParentHUD_C|GetWBP_KeyAdded _parenthudref))
  (bind _wbp_keyaddedbedroom (Variables|/Game/UserInterface/Player/HUD/WBP_ParentHUD.WBP_ParentHUD_C|GetWBP_KeyAddedBedroom _parenthudref_2))
  (Utilities|Array|AddUnique (Variables|Default|GetKeyRing) KeyID)
  (if (== KeyID 25)
    (Widget|SetVisibility _wbp_keyaddedbedroom "Visible")
    (Default|BedroomKeyAddedAnimation _wbp_keyaddedbedroom)
    (else
      (Widget|SetVisibility _wbp_keyadded "Visible")
      (Default|KeyAddedAnimation _wbp_keyadded))))

(event Custom|AddNote2
  (bind _returnvalue (Game|GetPlayerController 0))
  (bind _returnvalue_2 (UserInterface|CreateWidget "/Game/UserInterface/Screens/WBP_Note2.WBP_Note2_C"))
  (UserInterface|Viewport|AddtoViewport _returnvalue_2 0)
  (Variables|/Script/Engine.PlayerController|SetbShowMouseCursor _returnvalue true)
  (Input|SetInputModeUIOnly _returnvalue 0 "DoNotLock" false))

(event Custom|AddNote
  (bind _returnvalue (Game|GetPlayerController 0))
  (bind _returnvalue_2 (UserInterface|CreateWidget "/Game/UserInterface/Screens/WBP_Note.WBP_Note_C"))
  (UserInterface|Viewport|AddtoViewport _returnvalue_2 0)
  (Variables|/Script/Engine.PlayerController|SetbShowMouseCursor _returnvalue true)
  (Input|SetInputModeUIOnly _returnvalue 0 "DoNotLock" false))

(event Input|EnhancedActionEvents|EnhancedInputActionIA_Pause
  (params (ActionValue :type Boolean) (ElapsedSeconds :type Float%20%28double-precision%29) (TriggeredSeconds :type Float%20%28double-precision%29) (InputAction :type Input%20Action%20Object%20Reference :default "/Game/Player/Input/Actions/IA_Pause.IA_Pause"))
  (bind _returnvalue (Game|GetPlayerController 0))
  (:Started
    (if (not (Variables|UI|GetPauseOn))
      (Game|SetGamePaused true)
      (Variables|UI|SetPauseOn true)
      (Viewport|RemoveAllWidgets)
      (bind _returnvalue_2 (UserInterface|CreateWidget "/Game/UserInterface/Screens/WBP_PauseMenu.WBP_PauseMenu_C"))
      (UserInterface|Viewport|AddtoViewport _returnvalue_2 0)
      (Variables|/Script/Engine.PlayerController|SetbShowMouseCursor _returnvalue true)
      (Input|SetInputModeUIOnly _returnvalue 0 "DoNotLock" false))))

(event Input|EnhancedActionEvents|EnhancedInputActionIA_Move
  (params (ActionValue :type Vector%202D%20Structure) (ElapsedSeconds :type Float%20%28double-precision%29) (TriggeredSeconds :type Float%20%28double-precision%29) (InputAction :type Input%20Action%20Object%20Reference :default "/Game/Player/Input/Actions/IA_Move.IA_Move"))
  (:Triggered
    (CallFunction|ShouldStopSprint (.y ActionValue))))

(event EventBeginPlay
  (Variables|/Game/ActorComponents/Weapons/BPC_Gun.BPC_Gun_C|SetItemType (Variables|/Game/Holdables/Weapons/BP_WeaponBase.BP_WeaponBase_C|GetBPC_Gun (CallFunction|GetWeapon)) "NewEnumerator0")
  (bind _output_get (Variables|Health|SetHealthCurrent (Variables|Health|GetHealthMax)))
  (Development|PrintString (Utilities|String|ToString(Float) _output_get))
  (bind _returnvalue (UserInterface|CreateWidget "/Game/UserInterface/Player/HUD/WBP_ParentHUD.WBP_ParentHUD_C"))
  (bind _output_get_2 (Variables|UI|SetParentHUDRef _returnvalue))
  (UserInterface|Viewport|AddtoViewport _output_get_2 0))

(event Game|Damage|EventAnyDamage
  (params (Damage :type Float%20%28single-precision%29) (DamageType :type Damage%20Type%20Object%20Reference) (InstigatedBy :type Controller%20Object%20Reference) (DamageCauser :type Actor%20Object%20Reference))
  (bind _parenthudref (Variables|UI|GetParentHUDRef))
  (bind _wbp_healtheffect (Variables|/Game/UserInterface/Player/HUD/WBP_ParentHUD.WBP_ParentHUD_C|GetWBP_HealthEffect _parenthudref))
  (Variables|Health|SetHealthCurrent (Math|Float|Clamp(Float) (- (Variables|Health|GetHealthCurrent) Damage) 0.0 (Variables|Health|GetHealthMax)))
  (Widget|SetVisibility _wbp_healtheffect "Visible")
  (Default|HealthEffect _wbp_healtheffect)
  (if (<= (Variables|Health|GetHealthCurrent) 0.0)
    (CallFunction|Dead)))

(event Input|KeyboardEvents|DebugKeyT
  (params (Key :type Key%20Structure :default "None") (ActionValue :type Input%20Action%20Value%20Structure))
  (:Pressed
    (Game|Damage|ApplyDamage self 25.0 0 0)))

(event Input|KeyboardEvents|E
  (params (Key :type Key%20Structure :default "None")))

(fn ConstructionScript)

(fn TrytoStandUp
  (bind _returnvalue (Transformation|GetActorLocation))
  (bind _returnvalue_2 (Transformation|GetActorLocation))
  (bind _returnvalue_3 (Collision|MultiSphereTraceByChannel (Math|Vector|MakeVector (.x _returnvalue_2) (.y _returnvalue_2) (+ (.z _returnvalue_2) (Variables|CharacterVariables|GetCrouchHeight))) (Math|Vector|MakeVector (.x _returnvalue) (.y _returnvalue) (* (+ (.z _returnvalue) (Variables|CharacterVariables|GetStandHeight)) 1.1)) (Variables|/Script/Engine.CapsuleComponent|GetCapsuleRadius (Variables|Default|GetCapsuleComponent)) "TraceTypeQuery1" false (Utilities|Array|MakeArray self) "None"))
  (if (not _returnvalue_3)
    (CallFunction|StandUp)
    (Utilities|Time|ClearandInvalidateTimerbyHandle (Variables|Crouch|GetUnCrouchTimer))))

(fn CalculateLagVec
  (bind _returnvalue (Transformation|GetVelocity))
  (bind _basewalkspeed (Variables|CharacterVariables|GetBaseWalkSpeed))
  (Variables|Walking|SetLocationLagVec (Math|Interpolation|VInterpTo (Variables|Walking|GetLocationLagVec) (Math|Vector|ClampVectorSize (* (Math|Vector|MakeVector (/ (Math|Vector|DotProduct _returnvalue (Transformation|GetActorRightVector)) _basewalkspeed) (/ (Math|Vector|DotProduct _returnvalue (Transformation|GetActorForwardVector)) (* _basewalkspeed -1.0)) (/ (Math|Vector|DotProduct _returnvalue (Transformation|GetActorUpVector)) (* (Variables|/Script/Engine.CharacterMovementComponent|GetJumpZVelocity (Variables|Character|GetCharacterMovement)) -1.0))) 2.0) 0.0 4.0) (Utilities|Time|GetWorldDeltaSeconds) (/ (/ 1.0 (Utilities|Time|GetWorldDeltaSeconds)) 6.0))))

(fn GetWeapon
  (bind _asbp_weapon_base (Utilities|Casting|CastToBP_WeaponBase (Variables|/Script/Engine.ChildActorComponent|GetChildActor (Variables|Default|GetWeapon))))
  (return _asbp_weapon_base))

(fn SetItem
  (params (ItemType :type E_ItemType%20Enum :default "NewEnumerator3") (ObjectRef :type BP%20Interactable%20Base%20Object%20Reference))
  (switch Utilities|FlowControl|Switch|SwitchonE_ItemType ItemType
    (:NewEnumerator0
      (Variables|Item|SetWeaponObject "/Game/Holdables/Weapons/Guns/RetributionGun/BP_RetributionGun.BP_RetributionGun_C"))
    (:NewEnumerator1
      (Variables|Item|SetWeaponObject "/Game/Holdables/Weapons/Knives/Knife1/BP_Knife1.BP_Knife1_C"))
    (:NewEnumerator2
      (Variables|Item|SetWeaponObject "/Game/Holdables/BP_TestItem.BP_TestItem_C"))
    (:NewEnumerator4
      (Variables|Weapons|SetAmmoCount (+ (Variables|Weapons|GetAmmoCount) (Variables|/Game/Interactables/BP_InteractableBase.BP_InteractableBase_C|GetAmmoSize ObjectRef))))
    (:NewEnumerator6
      (Variables|Item|SetWeaponObject "/Game/Holdables/Weapons/Items/Lantern/BP_Lantern.BP_Lantern_C"))
    (:NewEnumerator7
      (Variables|Item|SetWeaponObject "/Game/Holdables/Weapons/Items/Mask/BP_Mask.BP_Mask_C"))
    (:NewEnumerator8
      (Variables|Item|SetWeaponObject "/Game/Holdables/Weapons/Items/Medkit/BP_Medkit.BP_Medkit_C")))
  (return))

(fn ReAlignWeapon
  (params (ItemType :type E_ItemType%20Enum :default "NewEnumerator3"))
  (bind _weapon (Variables|Default|GetWeapon))
  (bind _weapon_2 (Variables|Default|GetWeapon))
  (bind _weapon_3 (Variables|Default|GetWeapon))
  (bind _weapon_4 (Variables|Default|GetWeapon))
  (bind _weapon_5 (Variables|Default|GetWeapon))
  (bind _weapon_6 (Variables|Default|GetWeapon))
  (Development|SetHiddeninGame (Variables|Default|GetFirstPersonMesh) true false)
  (switch Utilities|FlowControl|Switch|SwitchonE_ItemType ItemType
    (:NewEnumerator0
      (Transformation|AttachComponentToComponent _weapon_2 (Variables|Default|GetFirstPersonMesh) "socket_gun" "KeepRelative" "KeepRelative" "KeepRelative" true)
      (ChildActorComponent|SetChildActorClass _weapon_2 "/Game/Holdables/Weapons/Guns/RetributionGun/BP_RetributionGun.BP_RetributionGun_C")
      (Variables|/Game/ActorComponents/Weapons/BPC_Gun.BPC_Gun_C|SetCurrentAmmo (Variables|/Game/Holdables/Weapons/BP_WeaponBase.BP_WeaponBase_C|GetBPC_Gun (CallFunction|GetWeapon)) (Variables|Weapons|GetTempAmmoVal))
      (Variables|/Game/Holdables/Weapons/BP_WeaponBase.BP_WeaponBase_C|SetItemType (CallFunction|GetWeapon) "NewEnumerator0")
      (Widget|SetVisibility (Variables|/Game/UserInterface/Player/HUD/WBP_ParentHUD.WBP_ParentHUD_C|GetWBP_GunMag (Variables|UI|GetParentHUDRef)) "Visible")
      (Widget|SetVisibility (Variables|/Game/UserInterface/Player/HUD/WBP_ParentHUD.WBP_ParentHUD_C|GetWBP_CrossHair (Variables|UI|GetParentHUDRef)) "Visible"))
    (:NewEnumerator1
      (Transformation|AttachComponentToComponent _weapon (Variables|Default|GetFirstPersonMesh) "socket_melee" "KeepRelative" "KeepRelative" "KeepRelative" true)
      (ChildActorComponent|SetChildActorClass _weapon "/Game/Holdables/Weapons/Knives/Knife1/BP_Knife1.BP_Knife1_C")
      (Variables|/Game/Holdables/Weapons/BP_WeaponBase.BP_WeaponBase_C|SetItemType (CallFunction|GetWeapon) "NewEnumerator1")
      (Widget|SetVisibility (Variables|/Game/UserInterface/Player/HUD/WBP_ParentHUD.WBP_ParentHUD_C|GetWBP_GunMag (Variables|UI|GetParentHUDRef)) "Hidden" :!label _label)
      (Widget|SetVisibility (Variables|/Game/UserInterface/Player/HUD/WBP_ParentHUD.WBP_ParentHUD_C|GetWBP_CrossHair (Variables|UI|GetParentHUDRef)) "Hidden"))
    (:NewEnumerator2
      (Transformation|AttachComponentToComponent _weapon_5 (Variables|Default|GetFirstPersonMesh) "socket_melee" "KeepRelative" "KeepRelative" "KeepRelative" true)
      (ChildActorComponent|SetChildActorClass _weapon_5 "/Game/Holdables/BP_TestItem.BP_TestItem_C")
      (Variables|/Game/Holdables/Weapons/BP_WeaponBase.BP_WeaponBase_C|SetItemType (CallFunction|GetWeapon) "NewEnumerator2")
      (goto _label))
    (:NewEnumerator6
      (Transformation|AttachComponentToComponent _weapon_6 (Variables|Default|GetFirstPersonMesh) "hand_r" "KeepRelative" "KeepRelative" "KeepRelative" true)
      (ChildActorComponent|SetChildActorClass _weapon_6 "/Game/Holdables/Weapons/Items/Lantern/BP_Lantern.BP_Lantern_C")
      (Variables|/Game/Holdables/Weapons/BP_WeaponBase.BP_WeaponBase_C|SetItemType (CallFunction|GetWeapon) "NewEnumerator6")
      (goto _label))
    (:NewEnumerator7
      (Transformation|AttachComponentToComponent _weapon_3 (Variables|Default|GetFirstPersonMesh) "socket_gun" "KeepRelative" "KeepRelative" "KeepRelative" true)
      (ChildActorComponent|SetChildActorClass _weapon_3 "/Game/Holdables/Weapons/Items/Mask/BP_Mask.BP_Mask_C")
      (Variables|/Game/Holdables/Weapons/BP_WeaponBase.BP_WeaponBase_C|SetItemType (CallFunction|GetWeapon) "NewEnumerator7")
      (goto _label))
    (:NewEnumerator8
      (Transformation|AttachComponentToComponent _weapon_4 (Variables|Default|GetFirstPersonMesh) "socket_medkit" "KeepRelative" "KeepRelative" "KeepRelative" true)
      (ChildActorComponent|SetChildActorClass _weapon_4 "/Game/Holdables/Weapons/Items/Medkit/BP_Medkit.BP_Medkit_C")
      (Variables|/Game/Holdables/Weapons/BP_WeaponBase.BP_WeaponBase_C|SetItemType (CallFunction|GetWeapon) "NewEnumerator8")
      (goto _label))))

(fn ItemCycleDown
  (if (== (Variables|Weapons|GetCurrentWeaponIndex) 0)
    (Variables|Weapons|SetCurrentWeaponIndex (- (Utilities|Array|Length (Variables|Weapons|GetWeaponClass)) 1))
    (else
      (Math|Integer|DecrementInt (Variables|Weapons|GetCurrentWeaponIndex)
        (:%20%20
          _))))
  (return))

(fn ItemCycleUp
  (if (== (Variables|Weapons|GetCurrentWeaponIndex) (- (Utilities|Array|Length (Variables|Weapons|GetWeaponClass)) 1))
    (Variables|Weapons|SetCurrentWeaponIndex 0)
    (else
      (Math|Integer|IncrementInt (Variables|Weapons|GetCurrentWeaponIndex)
        (:%20%20
          _))))
  (return))

(event Custom|Dip
  (params (Speed :type Float%20%28double-precision%29) (Strength :type Float%20%28double-precision%29))
  (bind _fp_root (Variables|Default|GetFP_Root))
  (bind _relativelocation (Variables|/Script/Engine.SceneComponent|GetRelativeLocation _fp_root))
  ;[1 1 1] Dip Event - An event that shakes the body when the character jumps or lands
  (Components|Timeline|SetPlayRate (Variables|Default|GetTL_Dip) Speed)
  (Variables|Dip|SetDipStrength Strength)
  (bind _dipalpha (Timeline|TL_Dip PlayFromStart)
    (:Update
      (Variables|Dip|SetDipAlpha (* _dipalpha (Variables|Dip|GetDipStrength)))
      (Transformation|SetRelativeLocation (Variables|Default|GetFP_Root) (Math|Vector|MakeVector (.x _relativelocation) (.y _relativelocation) (Math|Float|Lerp 0.0 -1e+01 (Variables|Dip|GetDipAlpha))) false false))))

(event Custom|JumpDip
  ;[1 1 1] Dip Event - An event that shakes the body when the character jumps or lands
  ;;[1 1 1] Jumping Landing Dip
  (CallFunction|Dip 4.0 0.5)
  (Audio|PlaySoundatLocation 0 (Transformation|GetActorLocation) "0, 0, 0" 1.0 1.0 0.0 0 0 0 0))

(event Custom|LandDip
  (bind _charactermovement (Variables|Character|GetCharacterMovement))
  ;[1 1 1] Dip Event - An event that shakes the body when the character jumps or lands
  ;;[1 1 1] Jumping Landing Dip
  (CallFunction|Dip 5.0 (Math|Float|Clamp(Float) (Math|Float|NormalizetoRange (Math|Vector|VectorLength (Math|Vector|MakeVector 0.0 0.0 (.z (Pawn|Components|CharacterMovement|GetLastUpdateVelocity _charactermovement)))) 0.0 (Variables|/Script/Engine.CharacterMovementComponent|GetJumpZVelocity _charactermovement)) 0.0 2.0))
  (Audio|PlaySoundatLocation 0 (Transformation|GetActorLocation) "0, 0, 0" 1.0 1.0 0.0 0 0 0 0))

(event EventOnJumped
  ;[1 1 1] Dip Event - An event that shakes the body when the character jumps or lands
  ;;[1 1 1] Jumping Landing Dip
  (CallFunction|JumpDip))

(event EventOnLanded
  (params (Hit :type Hit%20Result%20Structure%20%28by%20ref%29))
  ;[1 1 1] Dip Event - An event that shakes the body when the character jumps or lands
  ;;[1 1 1] Jumping Landing Dip
  (CallFunction|LandDip))

(event Custom|StandUp
  (bind _basewalkspeed (Variables|CharacterVariables|GetBaseWalkSpeed))
  (Variables|CharacterVariables|SetMovement "NewEnumerator0")
  (Utilities|FlowControl|Sequence
    (:then_0
      (bind _crouchalpha (Timeline|TL_Crouch Reverse)
        (:Update
          (Variables|Crouch|SetCrouchAlpha _crouchalpha)
          (switch Utilities|FlowControl|Switch|SwitchonE_MovementMode (Variables|CharacterVariables|GetMovement)
            (:NewEnumerator0
              (Variables|/Script/Engine.CharacterMovementComponent|SetMaxWalkSpeed (Variables|Character|GetCharacterMovement) (Math|Float|Lerp _basewalkspeed (* _basewalkspeed 0.5) (Variables|Crouch|GetCrouchAlpha)) :!label _label))
            (:NewEnumerator1
              (goto _label))
            (:NewEnumerator2
              _))
          (Components|Capsule|SetCapsuleHalfHeight (Variables|Default|GetCapsuleComponent) (Math|Float|Lerp (Variables|CharacterVariables|GetStandHeight) (Variables|CharacterVariables|GetCrouchHeight) (Variables|Crouch|GetCrouchAlpha)) true))))
    (:then_1
      (if (Variables|Sprint|GetSprintToggle)
        (CallFunction|StartSprint)))))

(event Input|EnhancedActionEvents|EnhancedInputActionIA_Crouch
  (params (ActionValue :type Boolean) (ElapsedSeconds :type Float%20%28double-precision%29) (TriggeredSeconds :type Float%20%28double-precision%29) (InputAction :type Input%20Action%20Object%20Reference :default "/Game/Player/Input/Actions/IA_Crouch.IA_Crouch"))
  (bind _basewalkspeed (Variables|CharacterVariables|GetBaseWalkSpeed))
  (:Started
    (Variables|Crouch|SetCrouchToggle true)
    (if (Utilities|Enum|Equal(Enum) (Variables|CharacterVariables|GetMovement) "NewEnumerator2")
      (CallFunction|StopSprint))
    (if (not (AI|Components|NavMovement|IsFalling (Variables|Character|GetCharacterMovement)))
      (Variables|CharacterVariables|SetMovement "NewEnumerator1")
      (Utilities|Time|ClearandInvalidateTimerbyHandle (Variables|Crouch|GetUnCrouchTimer))
      (bind _crouchalpha (Timeline|TL_Crouch Play)
        (:Update
          (Variables|Crouch|SetCrouchAlpha _crouchalpha)
          (switch Utilities|FlowControl|Switch|SwitchonE_MovementMode (Variables|CharacterVariables|GetMovement)
            (:NewEnumerator0
              (Variables|/Script/Engine.CharacterMovementComponent|SetMaxWalkSpeed (Variables|Character|GetCharacterMovement) (Math|Float|Lerp _basewalkspeed (* _basewalkspeed 0.5) (Variables|Crouch|GetCrouchAlpha)) :!label _label))
            (:NewEnumerator1
              (goto _label))
            (:NewEnumerator2
              _))
          (Components|Capsule|SetCapsuleHalfHeight (Variables|Default|GetCapsuleComponent) (Math|Float|Lerp (Variables|CharacterVariables|GetStandHeight) (Variables|CharacterVariables|GetCrouchHeight) (Variables|Crouch|GetCrouchAlpha)) true)))))
  (:Completed
    (Variables|Crouch|SetCrouchToggle false)
    (bind _returnvalue (Utilities|Time|SetTimerbyFunctionName 0 "TryToStandUp" 0.01 true))
    (Variables|Crouch|SetUnCrouchTimer _returnvalue)))

(event Custom|StartSprint
  (switch Utilities|FlowControl|Switch|SwitchonE_MovementMode (Variables|CharacterVariables|GetMovement)
    (:NewEnumerator0
      (Variables|CharacterVariables|SetMovement "NewEnumerator2")
      (Variables|/Script/Engine.CharacterMovementComponent|SetMaxWalkSpeed (Variables|Character|GetCharacterMovement) (* (Variables|CharacterVariables|GetBaseWalkSpeed) 1.5)))))

(event Custom|ShouldStopSprint
  (params (VelocityAxis :type Float%20%28double-precision%29))
  (if (< VelocityAxis 0.5)
    (switch Utilities|FlowControl|Switch|SwitchonE_MovementMode (Variables|CharacterVariables|GetMovement)
      (:NewEnumerator2
        (Variables|CharacterVariables|SetMovement "NewEnumerator0")
        (Variables|/Script/Engine.CharacterMovementComponent|SetMaxWalkSpeed (Variables|Character|GetCharacterMovement) (Variables|CharacterVariables|GetBaseWalkSpeed))))))

(event Custom|StopSprint
  (switch Utilities|FlowControl|Switch|SwitchonE_MovementMode (Variables|CharacterVariables|GetMovement)
    (:NewEnumerator2
      (Variables|CharacterVariables|SetMovement "NewEnumerator0")
      (Variables|/Script/Engine.CharacterMovementComponent|SetMaxWalkSpeed (Variables|Character|GetCharacterMovement) (Variables|CharacterVariables|GetBaseWalkSpeed)))))

(event Input|EnhancedActionEvents|EnhancedInputActionIA_Sprint
  (params (ActionValue :type Boolean) (ElapsedSeconds :type Float%20%28double-precision%29) (TriggeredSeconds :type Float%20%28double-precision%29) (InputAction :type Input%20Action%20Object%20Reference :default "/Game/Player/Input/Actions/IA_Sprint.IA_Sprint"))
  (:Started
    (Variables|Sprint|SetSprintToggle true)
    (switch Utilities|FlowControl|Switch|SwitchonE_MovementMode (Variables|CharacterVariables|GetMovement)
      (:NewEnumerator0
        (Variables|CharacterVariables|SetMovement "NewEnumerator2")
        (Variables|/Script/Engine.CharacterMovementComponent|SetMaxWalkSpeed (Variables|Character|GetCharacterMovement) (* (Variables|CharacterVariables|GetBaseWalkSpeed) 1.5)))))
  (:Completed
    (Variables|Sprint|SetSprintToggle false)
    (switch Utilities|FlowControl|Switch|SwitchonE_MovementMode (Variables|CharacterVariables|GetMovement)
      (:NewEnumerator2
        (Variables|CharacterVariables|SetMovement "NewEnumerator0")
        (Variables|/Script/Engine.CharacterMovementComponent|SetMaxWalkSpeed (Variables|Character|GetCharacterMovement) (Variables|CharacterVariables|GetBaseWalkSpeed))))))

(event Input|EnhancedActionEvents|EnhancedInputActionIA_PrimaryAction
  (params (ActionValue :type Boolean) (ElapsedSeconds :type Float%20%28double-precision%29) (TriggeredSeconds :type Float%20%28double-precision%29) (InputAction :type Input%20Action%20Object%20Reference :default "/Game/Player/Input/Actions/IA_PrimaryAction.IA_PrimaryAction"))
  (:Started
    (switch Utilities|FlowControl|Switch|SwitchonE_ItemType (Variables|/Game/Holdables/Weapons/BP_WeaponBase.BP_WeaponBase_C|GetItemType (CallFunction|GetWeapon))
      (:NewEnumerator0
        (|GunStarted))
      (:NewEnumerator1
        (|MeleeStarted))
      (:NewEnumerator2
        (Development|PrintString "Item Input"))
      (:NewEnumerator6
        (Development|PrintString "Lantern Input"))
      (:NewEnumerator7
        (Development|PrintString "Mask Input"))
      (:NewEnumerator8
        (Development|PrintString "Medkit Input")
        (Default|UseMedkit (Variables|/Game/Holdables/Weapons/BP_WeaponBase.BP_WeaponBase_C|GetBPC_Medkit (CallFunction|GetWeapon))))))
  (:Completed
    (switch Utilities|FlowControl|Switch|SwitchonE_ItemType (Variables|/Game/Holdables/Weapons/BP_WeaponBase.BP_WeaponBase_C|GetItemType (CallFunction|GetWeapon))
      (:NewEnumerator0
        (|GunCompleted))
      (:NewEnumerator1
        (|MeleeCompleted))
      (:NewEnumerator2
        (Development|PrintString "Item Input Completed"))
      (:NewEnumerator6
        (Development|PrintString "Lantern Input Completed"))
      (:NewEnumerator7
        (Development|PrintString "Mask Input Completed"))
      (:NewEnumerator8
        (Development|PrintString "Medkit Input Completed")))))

(event Input|EnhancedActionEvents|EnhancedInputActionIA_Reload
  (params (ActionValue :type Boolean) (ElapsedSeconds :type Float%20%28double-precision%29) (TriggeredSeconds :type Float%20%28double-precision%29) (InputAction :type Input%20Action%20Object%20Reference :default "/Game/Player/Input/Actions/IA_Reload.IA_Reload"))
  (:Triggered
    (if (not (== (Variables|Weapons|GetAmmoCount) 0))
      (Default|Reload (Variables|/Game/Holdables/Weapons/BP_WeaponBase.BP_WeaponBase_C|GetBPC_Gun (CallFunction|GetWeapon))))))

(event Input|EnhancedActionEvents|EnhancedInputActionIA_Interact
  (params (ActionValue :type Boolean) (ElapsedSeconds :type Float%20%28double-precision%29) (TriggeredSeconds :type Float%20%28double-precision%29) (InputAction :type Input%20Action%20Object%20Reference :default "/Game/Player/Input/Actions/IA_Interact.IA_Interact"))
  (:Triggered
    (if (not (Variables|Item|GetPickedUp?))
      (bind _array_element (Utilities|Array|ForEachLoopwithBreak (Collision|GetOverlappingActors 0 :!class /Script/Engine.Actor) :!label _label)
        (:LoopBody
          (if (Utilities|DoesObjectImplementInterface _array_element "/Game/Interactables/Interface/BPI_Interact.BPI_Interact_C")
            (Class|BPIInteract|Interact(Message) _array_element)
            (bind _asbp_interactable_base (Utilities|Casting|CastToBP_InteractableBase _array_element))
            (CallFunction|SetItem (Variables|/Game/Interactables/BP_InteractableBase.BP_InteractableBase_C|GetItemType _asbp_interactable_base) _asbp_interactable_base)
            (Utilities|Array|AddUnique (Variables|Weapons|GetWeaponClass) (Variables|Item|GetWeaponObject))
            (CallFunction|ReAlignWeapon (Variables|/Game/Interactables/BP_InteractableBase.BP_InteractableBase_C|GetItemType _asbp_interactable_base))
            (goto _label Break)))))))

(event Input|EnhancedActionEvents|EnhancedInputActionIA_ItemCycleUP
  (params (ActionValue :type Boolean) (ElapsedSeconds :type Float%20%28double-precision%29) (TriggeredSeconds :type Float%20%28double-precision%29) (InputAction :type Input%20Action%20Object%20Reference :default "/Game/Player/Input/Actions/IA_ItemCycleUP.IA_ItemCycleUP"))
  (bind _currentweaponindex (Variables|Weapons|GetCurrentWeaponIndex))
  (bind _weaponclass (Variables|Weapons|GetWeaponClass))
  (:Triggered
    (if (or (not (Variables|/Game/ActorComponents/Weapons/BPC_Gun.BPC_Gun_C|GetReloading? (Variables|/Game/Holdables/Weapons/BP_WeaponBase.BP_WeaponBase_C|GetBPC_Gun (CallFunction|GetWeapon)))) false)
      (CallFunction|ItemCycleUp)
      (ChildActorComponent|SetChildActorClass (Variables|Default|GetWeapon) (Utilities|Array|Get(acopy) _weaponclass _currentweaponindex))
      (if (Utilities|Array|IsValidIndex _weaponclass _currentweaponindex)
        (CallFunction|ReAlignWeapon (Variables|/Game/Holdables/Weapons/BP_WeaponBase.BP_WeaponBase_C|GetItemType (CallFunction|GetWeapon)))))))

(event Input|EnhancedActionEvents|EnhancedInputActionIA_ItemCycleDown
  (params (ActionValue :type Boolean) (ElapsedSeconds :type Float%20%28double-precision%29) (TriggeredSeconds :type Float%20%28double-precision%29) (InputAction :type Input%20Action%20Object%20Reference :default "/Game/Player/Input/Actions/IA_ItemCycleDown.IA_ItemCycleDown"))
  (bind _currentweaponindex (Variables|Weapons|GetCurrentWeaponIndex))
  (bind _weaponclass (Variables|Weapons|GetWeaponClass))
  (:Triggered
    (if (or (not (Variables|/Game/ActorComponents/Weapons/BPC_Gun.BPC_Gun_C|GetReloading? (Variables|/Game/Holdables/Weapons/BP_WeaponBase.BP_WeaponBase_C|GetBPC_Gun (CallFunction|GetWeapon)))) false)
      (CallFunction|ItemCycleDown)
      (ChildActorComponent|SetChildActorClass (Variables|Default|GetWeapon) (Utilities|Array|Get(acopy) _weaponclass _currentweaponindex))
      (if (Utilities|Array|IsValidIndex _weaponclass _currentweaponindex)
        (CallFunction|ReAlignWeapon (Variables|/Game/Holdables/Weapons/BP_WeaponBase.BP_WeaponBase_C|GetItemType (CallFunction|GetWeapon)))))))

(event Custom|Dead
  (Game|SetGamePaused true)
  (Viewport|RemoveAllWidgets)
  (bind _returnvalue (UserInterface|CreateWidget "/Game/UserInterface/Screens/WBP_GAMEOVER.WBP_GAMEOVER_C"))
  (UserInterface|Viewport|AddtoViewport _returnvalue 0))