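; Base Blueprint for a sword-wielding Maskerader AI character, providing attack, weapon, patrol route and movement speed functions.
; Montages drive attacking, drawing and sheathing; notifies spawn the sword onto a hand socket or destroy it, and dispatchers report when montages end.
; SetMovementSpeed maps movement states to walk speeds.
; BeginPlay calls an empty ChasePlayer; the move-to-player attack loop is disconnected.
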(event `self.ReceiveBeginPlay`
  (`self.Chase Player`))

(event `Chase Player`)

(event `Attack`
  (`|PlayMontage` (`self.Mesh`) "/Game/Maskerader/Anims/Stable_Sword_Outward_Slash_Montage.Stable_Sword_Outward_Slash_Montage"
    (:`OnCompleted`
      _)
    (:`OnInterrupted`
      _))
  (`self.On attack end`))

(event `WeildSword`
  (bind _notifyname (`|PlayMontage` (`self.Mesh`) "/Game/Maskerader/Anims/Withdrawing_Sword_Montage.Withdrawing_Sword_Montage")
    (:`OnCompleted`
      (`self.OnWeildSword`))
    (:`OnNotifyBegin`
      (switch `name` _notifyname
        (:`CreateWeapon`
          (bind _returnvalue (`|SpawnActorFromClass` "/Game/Maskerader/Weapons/Sword_BP.Sword_BP_C" (`self.GetTransform`) "Undefined" "MultiplyWithRoot" null null))
          (bind _output_get (set `self.Sword` _returnvalue))
          (`self.K2_AttachToComponent` _output_get (`self.Mesh`) "RightHand_Sword" "SnapToTarget" "SnapToTarget" "SnapToTarget" true)
          (set `self.IsWeildingSword` true))))))

(event `RemoveSword`
  (bind _notifyname (`|PlayMontage` (`self.Mesh`) "/Game/Maskerader/Anims/Sheathing_Sword_Montage.Sheathing_Sword_Montage")
    (:`OnCompleted`
      (`self.OnDestroySword`))
    (:`OnNotifyBegin`
      (switch `name` _notifyname
        (:`DestroyWeapon`
          (`self.K2_DestroyActor` (`self.Sword`))
          (set `self.IsWeildingSword` false))))))

(fn `GetPatrolRoute`
  (returns (PatroleRoute :type "/Game/AI/PatrolRoute_BP Object Reference"))
  (return (`self.PatroleRoute`)))

(fn `SetMovementSpeed`
  (params (Speed :type "/Game/AI/Enums/MovementSpeed_E Enum" :default "NewEnumerator0"))
  (returns (SpeedValue :type "Float (double-precision)"))
  (bind _output_get (set `CharacterMovementComponent.MaxWalkSpeed` (select `/Game/AI/Enums/MovementSpeed_E` Speed :`NewEnumerator1` 150.0 :`NewEnumerator2` 300.0 :`NewEnumerator3` 500.0 :!type "Float (single-precision)") (`self.CharacterMovement`)))
  (return _output_get))

(fn `UserConstructionScript`)