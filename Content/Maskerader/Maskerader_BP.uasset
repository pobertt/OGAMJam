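; Maskerader_BP is a dancing character that reacts with surprise the first time it spots the player.
; On BeginPlay its mesh loops a Macarena dance animation.
; PawnSensing's OnSeePawn casts the seen pawn to BP_PlayerCharacter, and a match sets the SeenYou flag and plays a one-shot Surprised animation.
; SeenYou is never reset here, so the reaction happens once, and debug strings print for player and non-player sightings until then.
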(event `self.ReceiveBeginPlay`
  (`SkeletalMeshComponent.PlayAnimation` (`self.Mesh`) "/Game/Maskerader/Anims/Macarena_Dance.Macarena_Dance" true))

(event `self.PawnSensing.OnSeePawn`
  (params (Pawn :type "Pawn Object Reference"))
  (if (not (`self.SeenYou`))
    (cast `/Game/Player/BP_PlayerCharacter` Pawn
      (:`then`
        (`KismetSystemLibrary.PrintString` "I see you")
        (set `self.SeenYou` true)
        (`SkeletalMeshComponent.PlayAnimation` (`self.Mesh`) "/Game/Maskerader/Anims/Surprised.Surprised" false))
      (:`CastFailed`
        (`KismetSystemLibrary.PrintString` "naa")))))

(fn `UserConstructionScript`)